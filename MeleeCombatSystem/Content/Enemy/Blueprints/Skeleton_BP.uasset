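; Skeleton enemy character that runs a behavior tree and fights the player with a sword spawned onto its hand socket and linked to a trace component.
; Pawn sensing, damage and sphere-exit events update a behaviour enum mirrored to the blackboard.
; Damage plays a hit reaction with a retriggerable recovery delay, or at zero health stops AI, plays death and releases player lock-on.
; It also plays random attack montages and toggles a lock-on marker.
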(event `self.ReceiveBeginPlay`
  ;[1 1 1] Set up Enemy Character
  (`AIController.RunBehaviorTree` (`AIBlueprintHelperLibrary.GetAIController` self) "/Game/Enemy/BehaviourTree/Skeleton_BT.Skeleton_BT")
  (bind _returnvalue (`|SpawnActorFromClass` (`self.sword`) (`SceneComponent.GetSocketTransform` (`self.Mesh`) "sword" "RTS_World") "Undefined" "MultiplyWithRoot" null null))
  (bind _asbase_sword_bp (cast `/Game/Equipment/BaseSword_BP` _returnvalue))
  (bind _output_get (set `self.swordRef` _asbase_sword_bp))
  (`self.K2_AttachToComponent` _output_get (`self.Mesh`) "sword" "SnapToTarget" "SnapToTarget" "SnapToTarget" true)
  (set `/Game/Equipment/TraceComponent.SwordRef` (`self.swordRef`) (`self.TraceComponent`))
  (bind _asbp_third_person_character (cast `/Game/ThirdPerson/Blueprints/BP_ThirdPersonCharacter` (`GameplayStatics.GetPlayerCharacter` 0)))
  (set `self.PlayerRef` _asbp_third_person_character)
  (`BlackboardComponent.SetValueAsEnum` (`AIBlueprintHelperLibrary.GetBlackboard` null) "eBahaviour" (`self.behaviour`))
  (set `/Game/Equipment/RotatingComponent.Target` (`GameplayStatics.GetPlayerCharacter` 0) (`self.RotatingComponent`)))

(event `self.ReceiveAnyDamage`
  (params (Damage :type "Float (single-precision)") (DamageType :type "DamageType Object Reference") (InstigatedBy :type "Controller Object Reference") (DamageCauser :type "Actor Object Reference"))
  (bind _targetactor (`/Game/ThirdPerson/Blueprints/BP_ThirdPersonCharacter.TargetActor` (`self.PlayerRef`)))
  ;[1 1 1] Damage System
  (set `self.behaviour` "NewEnumerator0")
  (`BlackboardComponent.SetValueAsEnum` (`AIBlueprintHelperLibrary.GetBlackboard` null) "eBahaviour" (`self.behaviour`))
  (bind _output_get (set `self.Health` (- (`self.Health`) Damage)))
  (if (<= _output_get 0.0)
    (`/Engine/EditorBlueprintResources/StandardMacros.DoOnce` false
      (:`Completed`
        (`BrainComponent.StopLogic` (`AIController.BrainComponent` (`AIBlueprintHelperLibrary.GetAIController` self)) "die")
        (set `self.EnemyDead` true)
        (`self.PlayAnimMontage` "/Game/Enemy/Animations/SkeleDeath_Montage.SkeleDeath_Montage")
        (`/Engine/EditorBlueprintResources/StandardMacros.IsValid` _targetactor
          (:`Is Valid`
            (if (== _targetactor self)
              (`/Game/ThirdPerson/Blueprints/BP_ThirdPersonCharacter.DisengageLockon` (`self.PlayerRef`)))))))
    (else
      (`self.PlayAnimMontage` "/Game/Enemy/Animations/Skele_Hit_Montage.Skele_Hit_Montage")
      (`KismetSystemLibrary.RetriggerableDelay` (`self.DamageTime`))
      (set `self.behaviour` "NewEnumerator3")
      (`BlackboardComponent.SetValueAsEnum` (`AIBlueprintHelperLibrary.GetBlackboard` null) "eBahaviour" (`self.behaviour`)))))

(event `/Game/Lockon/LockOnInterface.OnSelected`
  ;[1 1 1] Handle lockon
  (`SceneComponent.SetVisibility` (`self.Lockon`) true false))

(event `/Game/Lockon/LockOnInterface.OnDeselected`
  ;[1 1 1] Handle lockon
  (`SceneComponent.SetVisibility` (`self.Lockon`) false false))

(event `Attack`
  ;[1 1 1] Attack System
  (bind _returnvalue (`self.PlayAnimMontage` (`KismetArrayLibrary.Array_Random` (`self.AttackAnimations`))))
  (set `self.attackLength` _returnvalue))

(event `self.PawnSensing.OnSeePawn`
  (params (Pawn :type "Pawn Object Reference"))
  ;[1 1 1] Handle Enemy Vision
  (if (and (== Pawn (`GameplayStatics.GetPlayerCharacter` 0)) (`|EnumInequality` (`self.behaviour`) "NewEnumerator0"))
    (set `self.behaviour` "NewEnumerator3")
    (`BlackboardComponent.SetValueAsEnum` (`AIBlueprintHelperLibrary.GetBlackboard` null) "eBahaviour" (`self.behaviour`))))

(event `self.Sphere.OnComponentEndOverlap`
  (params (OverlappedComponent :type "PrimitiveComponent Object Reference") (OtherActor :type "Actor Object Reference") (OtherComp :type "PrimitiveComponent Object Reference") (OtherBodyIndex :type Integer))
  ;[1 1 1] Escape Enemy
  (cast `/Game/ThirdPerson/Blueprints/BP_ThirdPersonCharacter` OtherActor)
  (set `self.behaviour` "NewEnumerator1")
  (`BlackboardComponent.SetValueAsEnum` (`AIBlueprintHelperLibrary.GetBlackboard` null) "eBahaviour" (`self.behaviour`)))

(fn `isDead`
  (returns (isDead :type Boolean))
  (return (`self.EnemyDead`)))

(fn `UserConstructionScript`)